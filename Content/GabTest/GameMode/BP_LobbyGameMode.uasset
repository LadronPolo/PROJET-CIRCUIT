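; Lobby game mode that gives players sports car pawns and moves the session to a chosen map.
; BeginPlay shows the launch-game widget to the first player controller.
; SpawnPlayer replaces a controller's pawn with a possessed SportsCar_Pawn, placed at the PlayerStart indexed by current player count.
; FadeOut triggers each vehicle controller's map transition, while TravelTo saves the player count to the GameInstance, then runs servertravel.
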(event `TravelTo`
  (params (Map :type String))
  (`self.SetPlayerCount`)
  (`KismetSystemLibrary.ExecuteConsoleCommand` (`KismetStringLibrary.Concat_StrStr` "servertravel " Map) null))

(event `FadeOut`
  (for _array_element (`GameStateBase.PlayerArray` (`GameplayStatics.GetGameState`))
    (bind _asvehicle_player_controller (cast `/Game/GabTest/VehicleTemplate/Blueprints/VehiclePlayerController` (`PlayerState.GetPlayerController` _array_element)))
    (`/Game/GabTest/VehicleTemplate/Blueprints/VehiclePlayerController.TransitionMap` _asvehicle_player_controller)))

(event `self.ReceiveBeginPlay`
  (bind _returnvalue (`|CreateWidget` "/Game/GabTest/BluePrints/BP_LaunchGame.BP_LaunchGame_C" (`GameplayStatics.GetPlayerController` 0)))
  (`UserWidget.AddToViewport` _returnvalue 1))

(fn `FindPlayerSpwawn`
  (returns (Location :type "Transform Structure"))
  (bind _returnvalue (`self.GetNumPlayers` (`GameStateBase.AuthorityGameMode` (`GameplayStatics.GetGameState`))))
  (bind _outactors (`GameplayStatics.GetAllActorsOfClass` "/Script/Engine.PlayerStart"))
  (return (`self.GetTransform` (`|GetArrayItem` _outactors (- _returnvalue 1)))))

(fn `SetPlayerCount`
  (bind _asbp_game_instance (cast `/Game/GabTest/GameInstance/BP_GameInstance` (`GameplayStatics.GetGameInstance`)))
  (set `/Game/GabTest/GameInstance/BP_GameInstance.NumberOfPlayer` (`KismetArrayLibrary.Array_Length` (`GameStateBase.PlayerArray` (`GameplayStatics.GetGameState`))) _asbp_game_instance))

(fn `SpawnPlayer`
  (params (PlayerController :type "PlayerController Object Reference"))
  (returns (NewParam :type "Pawn Object Reference"))
  (bind _returnvalue (`Controller.K2_GetPawn` PlayerController))
  (`/Engine/EditorBlueprintResources/StandardMacros.IsValid` _returnvalue
    (:`Is Valid`
      (`self.K2_DestroyActor` _returnvalue))
    (:`Is Not Valid`
      _))
  (bind _location (`self.FindPlayerSpwawn`))
  (bind _returnvalue_2 (`|SpawnActorFromClass` "/Game/GabTest/VehicleTemplate/Blueprints/SportsCar/SportsCar_Pawn.SportsCar_Pawn_C" _location "Undefined" "OverrideRootScale" null null))
  (`Controller.Possess` PlayerController _returnvalue_2)
  (return _returnvalue_2))

(fn `UserConstructionScript`)