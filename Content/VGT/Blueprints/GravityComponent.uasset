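; Vehicle gravity component (VGT template) that keeps the owning vehicle aligned to the surface beneath it, as an alternative to real gravity.
; BeginPlay spawns attached marker actors as trace points plus a commander actor for input, and ignores vehicle collisions until clear of spawn.
; With real gravity off, Tick traces down ahead and below; when both hit the same component, it rotates to the surface normal and holds DistanceFromGround.
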(event `self.ReceiveBeginPlay`
  (bind _returnvalue (`Actor.GetComponentByClass` (`self.Actor`) "/Script/Engine.StaticMeshComponent"))
  ;[1 1 1] VGT - Vehicles Gravity Template - AC_VGT_GravityComponent
  (set `self.Actor` (`self.GetOwner`))
  (`/Engine/EditorBlueprintResources/StandardMacros.IsValid` _returnvalue
    (:`Is Valid`
      (set `self.Mesh` _returnvalue)
      ;;[1 1 1] Prevents vehicles from colliding when spawning out
      (`PrimitiveComponent.SetCollisionResponseToChannel` (`self.Mesh`) "ECC_Vehicle" "ECR_Ignore")
      (bind _aspawn (cast `Pawn` (`self.GetOwner`))
        (:`then`
          (if (`Pawn.IsLocallyControlled` _aspawn)
            (bind _asplayer_controller (cast `PlayerController` (`Pawn.GetController` _aspawn)))
            (else
              (`/Engine/EditorBlueprintResources/StandardMacros.IsValid` (`GameplayStatics.GetPlayerController` 0)
                (:`Is Valid`
                  _))))
          (set `self.PlayerController` _asplayer_controller))
        (:`CastFailed`
          _))
      (`PrimitiveComponent.SetEnableGravity` (`self.Mesh`) (`self.RealGravityOn`))
      (`self.VehiculeConfig`)
      (set `self.ReadyToGo` true)
      (set `self.SpawnLocation` (`SceneComponent.K2_GetComponentLocation` (`self.Mesh`)))
      ;;[1 1 1] Allow vehicles from colliding each others
      (`KismetSystemLibrary.Delay` 2.0 :!label _label)
      (if (> (`KismetMathLibrary.VSize` (- (`self.SpawnLocation`) (`SceneComponent.K2_GetComponentLocation` (`self.Mesh`)))) 1000.0)
        (`PrimitiveComponent.SetCollisionResponseToChannel` (`self.Mesh`) "ECC_Vehicle" "ECR_Block")
        (else
          (goto _label))))))

(event `SpringArmConfig`
  (bind _springarm (`self.SpringArm`))
  (bind _returnvalue (`Actor.GetComponentByClass` (`self.Actor`) "/Script/Engine.SpringArmComponent"))
  ;[1 1 1] VGT - Vehicles Gravity Template - AC_VGT_GravityComponent
  (`/Engine/EditorBlueprintResources/StandardMacros.IsValid` _returnvalue
    (:`Is Valid`
      (set `self.SpringArm` _returnvalue)
      (set `SpringArmComponent.bInheritPitch` true _springarm)
      (set `SpringArmComponent.bInheritRoll` true _springarm)
      (set `SpringArmComponent.bInheritYaw` true _springarm))))

(event `self.ReceiveTick`
  (params (DeltaSeconds :type "Float (single-precision)"))
  (bind _actor (`self.Actor`))
  (bind _distancefromground (`self.DistanceFromGround`))
  (bind _rootcomponent (`Actor.RootComponent` _actor))
  ;[1 1 1] VGT - Vehicles Gravity Template - AC_VGT_GravityComponent
  (if (and (`self.ReadyToGo`) (not (`self.RealGravityOn`)))
    ;;[1 1 1] Springboard Prope
    (bind _outactors (`GameplayStatics.GetAllActorsOfClass` "/Game/EtienneTest/DemoContent/VehicleTemplate/Blueprints/SportsCar/BP_SportsCar_Pawn.BP_SportsCar_Pawn_C"))
    (bind (_outhit _returnvalue) (`KismetSystemLibrary.LineTraceSingle` (`Actor.K2_GetActorLocation` (`self.ProbOrigin`)) (`Actor.K2_GetActorLocation` (`self.Probe`)) "TraceTypeQuery1" true _outactors "Persistent" true (struct :`R` 0.908198 :`B` 1.0 :`A` 1.0)))
    (if _returnvalue
      (`PrimitiveComponent.SetEnableGravity` (`self.Mesh`) (`self.RealGravityOn`))
      ;;[1 1 1] Gravity system
      (bind _outactors_2 (`GameplayStatics.GetAllActorsOfClass` "/Game/EtienneTest/DemoContent/VehicleTemplate/Blueprints/SportsCar/BP_SportsCar_Pawn.BP_SportsCar_Pawn_C"))
      (bind (_outhit_2 _returnvalue_2) (`KismetSystemLibrary.LineTraceSingle` (`Actor.K2_GetActorLocation` (`self.Ref`)) (`Actor.K2_GetActorLocation` (`self.GoBottom`)) "TraceTypeQuery1" true _outactors_2 "Persistent"))
      (if _returnvalue_2
        (bind (_bblockinghit _binitialoverlap _time _distance _location _impactpoint _normal _impactnormal _physmat _hitactor _hitcomponent) (`GameplayStatics.BreakHitResult` _outhit_2))
        (`/Engine/EditorBlueprintResources/StandardMacros.IsValid` _hitcomponent
          (:`Is Valid`
            (if (== (`.HitComponent` (`GameplayStatics.BreakHitResult` _outhit)) _hitcomponent)
              (`Actor.K2_SetActorRotation` _actor (`KismetMathLibrary.MakeRotFromZ` _normal) false)
              (bind _returnvalue_3 (`KismetMathLibrary.Vector_Distance` _location (`SceneComponent.K2_GetComponentLocation` (`self.Mesh`))))
              (if (< _returnvalue_3 _distancefromground)
                (bind _returnvalue_4 (- _distancefromground _returnvalue_3))
                (`SceneComponent.K2_AddWorldOffset` _rootcomponent (`KismetMathLibrary.MakeVector` 0.0 0.0 _returnvalue_4) false false)
                (else
                  (`SceneComponent.K2_AddWorldOffset` _rootcomponent (`KismetMathLibrary.MakeVector` 0.0 0.0 _returnvalue_4) false false))))))))))

(event `VehiculeConfig`
  ;[1 1 1] VGT - Vehicles Gravity Template - AC_VGT_GravityComponent
  ;;[1 1 1] Vehicle configuration
  (`self.RefInit`)
  (`self.GoBottomInit`)
  (`self.ProbeInit`)
  (`self.CommanderInit`))

(event `RefInit`
  (bind _ref (`self.Ref`))
  ;[1 1 1] VGT - Vehicles Gravity Template - AC_VGT_GravityComponent
  ;;[1 1 1] Vehicle configuration
  ;;;[1 1 1] Reference System initialisation
  (bind _returnvalue (`|SpawnActorFromClass` "/Game/VGT/Blueprints/VGTsubsystems/BP_Mark.BP_Mark_C" (`KismetMathLibrary.MakeTransform` (0.0 0.0 0.0)) "Undefined" "OverrideRootScale" null null))
  (set `self.Ref` _returnvalue)
  (`Actor.K2_AttachToActor` (`self.Ref`) (`self.Actor`) "None" "KeepRelative" "KeepWorld" "KeepWorld" true)
  (`Actor.K2_SetActorRelativeLocation` _ref (0.0 0.0 50.0) false true)
  (`Actor.K2_SetActorRelativeRotation` :`self` _ref))

(event `GoBottomInit`
  ;[1 1 1] VGT - Vehicles Gravity Template - AC_VGT_GravityComponent
  ;;[1 1 1] Vehicle configuration
  ;;;[1 1 1] GoBottom system init
  (bind _returnvalue (`|SpawnActorFromClass` "/Game/VGT/Blueprints/VGTsubsystems/BP_Mark.BP_Mark_C" (`KismetMathLibrary.MakeTransform` (0.0 0.0 0.0)) "Undefined" "OverrideRootScale" null null))
  (set `self.GoBottom` _returnvalue)
  (`Actor.K2_AttachToActor` (`self.GoBottom`) (`self.Ref`) "None" "KeepRelative" "KeepWorld" "KeepWorld" true)
  (`Actor.K2_SetActorRelativeLocation` (`self.GoBottom`) (`KismetMathLibrary.MakeVector` 0.0 0.0 (* (`self.GravityDistance`) -1.0)) false true))

(event `ProbeInit`
  ;[1 1 1] VGT - Vehicles Gravity Template - AC_VGT_GravityComponent
  ;;[1 1 1] Vehicle configuration
  ;;;[1 1 1] Springboard Probe system init
  (bind _returnvalue (`|SpawnActorFromClass` "/Game/VGT/Blueprints/VGTsubsystems/BP_Mark.BP_Mark_C" (`KismetMathLibrary.MakeTransform` (0.0 0.0 0.0)) "Undefined" "OverrideRootScale" null null))
  (set `self.ProbOrigin` _returnvalue)
  (`Actor.K2_AttachToActor` (`self.ProbOrigin`) (`self.Ref`) "None" "KeepRelative" "KeepRelative" "KeepWorld" true)
  (`Actor.K2_SetActorRelativeLocation` (`self.ProbOrigin`) (200.0 0.0 0.0) false true)
  (bind _returnvalue_2 (`|SpawnActorFromClass` "/Game/VGT/Blueprints/VGTsubsystems/BP_Mark.BP_Mark_C" (`KismetMathLibrary.MakeTransform` (0.0 0.0 0.0)) "Undefined" "OverrideRootScale" null null))
  (set `self.Probe` _returnvalue_2)
  (`Actor.K2_AttachToActor` (`self.Probe`) (`self.Ref`) "None" "KeepRelative" "KeepRelative" "KeepWorld" true)
  (`Actor.K2_SetActorRelativeLocation` (`self.Probe`) (`KismetMathLibrary.MakeVector` 200.0 0.0 (* (`self.GravityDistance`) -1.0)) false true))

(event `CommanderInit`
  ;[1 1 1] VGT - Vehicles Gravity Template - AC_VGT_GravityComponent
  ;;[1 1 1] Vehicle configuration
  ;;;[1 1 1] Commander initialisation - allow to give input to actor component
  (bind _returnvalue (`|SpawnActorFromClass` "/Game/VGT/Blueprints/VGTsubsystems/BP_VGT_VehiculeCommander.BP_VGT_VehiculeCommander_C" (`KismetMathLibrary.MakeTransform` (0.0 0.0 0.0)) "Undefined" "OverrideRootScale" null null))
  (set `/Game/VGT/Blueprints/VGTsubsystems/BP_VGT_VehiculeCommander.AC_VGT_GravityComponent` self _returnvalue))