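; BP_ItemBox is an item box visual that tumbles continuously, with no pickup logic in its graphs.
; BeginPlay gives the SMItemBox mesh a random starting rotation and random per-axis spin speeds, which Tick applies as delta-time-scaled local rotation.
; Holding F sets the materials' OpacityCTRL parameter to zero and releasing restores it to one, apparently as a debug preview of hiding the box.
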(event `Key|F`
  (params (Key :type "Key Structure"))
  (:`Pressed`
    (`MeshComponent.SetScalarParameterValueOnMaterials` (`self.SM_Item_Box`) "OpacityCTRL" 0.0))
  (:`Released`
    (`MeshComponent.SetScalarParameterValueOnMaterials` (`self.SM_Item_Box`) "OpacityCTRL" 1.0)))

(event `self.ReceiveBeginPlay`
  (`SceneComponent.K2_SetRelativeRotation` (`self.SM_Item_Box`) (`KismetMathLibrary.RandomRotator` false) false false)
  (set `self.Value1` (`KismetMathLibrary.RandomFloatInRange` 20.0 70.0))
  (set `self.Value2` (`KismetMathLibrary.RandomFloatInRange` 20.0 70.0))
  (set `self.Value3` (`KismetMathLibrary.RandomFloatInRange` 20.0 70.0)))

(event `self.ReceiveTick`
  (params (DeltaSeconds :type "Float (single-precision)"))
  (`SceneComponent.K2_AddLocalRotation` (`self.SM_Item_Box`) (`KismetMathLibrary.MakeRotator` (* DeltaSeconds (`self.Value1`)) (* DeltaSeconds (`self.Value2`)) (* DeltaSeconds (`self.Value3`))) false false))

(fn `UserConstructionScript`)