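; BP_RacingLine is an actor that draws a racing line as instanced meshes placed at a fixed step along a spline.
; The construction script adds the instances, rotates each to look at the next point, aligns the last to the spline's rotation, and prints the instance count.
; On BeginPlay it passes the instanced mesh component, mesh and spline to an Initialize call.
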(event `self.ReceiveBeginPlay`
  (`self.Initialize` (`self.InstancedStaticMesh`) (`self.Mesh`) (`self.Spline`)))

(fn `UserConstructionScript`
  (bind _instancedstaticmesh (`self.InstancedStaticMesh`))
  (bind _instancedstaticmesh_2 (`self.InstancedStaticMesh`))
  (bind _returnvalue (`InstancedStaticMeshComponent.GetInstanceCount` (`self.InstancedStaticMesh`)))
  (bind _returnvalue_2 (- _returnvalue 1))
  (bind _outinstancetransform (`InstancedStaticMeshComponent.GetInstanceTransform` _instancedstaticmesh _returnvalue_2 true))
  ;[1 1 1] Populating Mesh Along Spline
  (`StaticMeshComponent.SetStaticMesh` (`self.InstancedStaticMesh`) (`self.Mesh`))
  (for _index (range (+ (`KismetMathLibrary.FFloor` (/ (`SplineComponent.GetSplineLength` (`self.Spline`)) (`self.Step`))) 1))
    (bind _returnvalue_3 (`SplineComponent.GetLocationAtDistanceAlongSpline` (`self.Spline`) (* _index (`self.Step`)) "World"))
    (`InstancedStaticMeshComponent.AddInstance` (`self.InstancedStaticMesh`) (`KismetMathLibrary.Conv_VectorToTransform` _returnvalue_3) true)
    (if (> _index 0)
      (bind _returnvalue_4 (- _index 1))
      (bind _outinstancetransform_2 (`InstancedStaticMeshComponent.GetInstanceTransform` _instancedstaticmesh_2 _returnvalue_4 true))
      (`InstancedStaticMeshComponent.UpdateInstanceTransform` _instancedstaticmesh_2 _returnvalue_4 (`KismetMathLibrary.MakeTransform` (.location _outinstancetransform_2) (`KismetMathLibrary.FindLookAtRotation` (.location _outinstancetransform_2) _returnvalue_3)) true false false)))
  (`KismetSystemLibrary.PrintString` (`KismetStringLibrary.Concat_StrStr` "Instance Count =" (`KismetStringLibrary.Conv_IntToString` _returnvalue)) true false (struct :`G` 0.66 :`B` 1.0 :`A` 1.0) 0.1)
  (`InstancedStaticMeshComponent.UpdateInstanceTransform` _instancedstaticmesh _returnvalue_2 (`KismetMathLibrary.MakeTransform` (.location _outinstancetransform) (`SplineComponent.FindRotationClosestToWorldLocation` (`self.Spline`) (.location _outinstancetransform) "World")) true false false))