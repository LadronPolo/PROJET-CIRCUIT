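; Player-controlled racing ship pawn with throttle, steering, drift, boost, items and timed effects like invincibility and miniaturization.
; Enhanced Input feeds wrapper and Local event pairs, apparently for networking, which call parent-class movement and item functions; boost briefly activates a physics thruster.
; Ordered checkpoint overlaps count laps, while Tick reports distance to the next checkpoint to the track GameMode.
; Player controllers receive HUD updates; finishing hides the ship and switches to spectating.
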(event `LocalUseItem`
  ;[1 1 1] Input
  (`AbilityPawn.UseItem`))

(event `SRUseItem`
  ;[1 1 1] Input
  (`self.LocalUseItem`))

(event `ChangeCamera`
  (params (pawn :type "Pawn Object Reference"))
  ;[1 1 1] Input
  (bind _asbp_track_game_mode (cast `/Game/Blueprint/GameMode/BP_TrackGameMode` (`GameplayStatics.GetGameMode`)))
  (bind _asbp_track_player_controller (cast `/Game/Blueprint/PlayerController/BP_TrackPlayerController` (`self.GetController` pawn)))
  (`/Game/Blueprint/GameMode/BP_TrackGameMode.FindCamera` _asbp_track_game_mode self (`/Game/Blueprint/PlayerController/BP_TrackPlayerController.currentSpect` _asbp_track_player_controller)))

(event `EnhancedInput|/Game/Blueprint/Input/Actions/IA_UseItem`
  (params (ActionValue :type Boolean) (ElapsedSeconds :type "Float (double-precision)") (TriggeredSeconds :type "Float (double-precision)") (InputAction :type "InputAction Object Reference" :default "/Game/Blueprint/Input/Actions/IA_UseItem.IA_UseItem"))
  ;[1 1 1] Input
  (:`Triggered`
    (bind _asbp_track_player_controller (cast `/Game/Blueprint/PlayerController/BP_TrackPlayerController` (`GameplayStatics.GetPlayerController` 0)))
    (`/Game/Blueprint/PlayerController/BP_TrackPlayerController.updateItem` _asbp_track_player_controller null)
    (`self.SRUseItem`)))

(event `EnhancedInput|/Game/Blueprint/Input/Actions/IA_Spectate`
  (params (ActionValue :type Boolean) (ElapsedSeconds :type "Float (double-precision)") (TriggeredSeconds :type "Float (double-precision)") (InputAction :type "InputAction Object Reference" :default "/Game/Blueprint/Input/Actions/IA_Spectate.IA_Spectate"))
  ;[1 1 1] Input
  (:`Started`
    (`self.ChangeCamera` self)))

(event `LocalDriftStart`
  ;[1 1 1] Input
  (`self.StartDrift`))

(event `LocalDriftEnd`
  ;[1 1 1] Input
  (`self.StopDrift`))

(event `lThrottle`
  (`self.AddMovementInput` (`self.GetActorForwardVector`)))

(event `DriftStart`
  ;[1 1 1] Input
  (`self.LocalDriftStart`))

(event `DriftEnd`
  ;[1 1 1] Input
  (`self.LocalDriftEnd`))

(event `LocalThrottle`
  (params (axis :type "Float (double-precision)"))
  (`self.Accelerate` 1.0))

(event `throttle`
  (params (axis :type "Float (double-precision)"))
  (`self.AddMovementInput` (`self.GetActorForwardVector`))
  (`self.lThrottle`))

(event `LocalActivateBoost`
  ;[1 1 1] Input
  (bind _returnvalue (`self.canBoost`))
  (bind _returnvalue_2 (`self.IsBoost`))
  (if (and _returnvalue (not _returnvalue_2))
    (`ActorComponent.SetActive` (`self.PhysicsThruster`) true false)
    (`self.spendBoost`)
    (`self.SetIsBoost` true)
    (`KismetSystemLibrary.Delay` (`self.boostDuration`))
    (`ActorComponent.SetActive` (`self.PhysicsThruster`) false false)
    (`self.SetIsBoost` false)))

(event `EnhancedInput|/Game/Blueprint/Input/Actions/IA_Handbrake`
  (params (ActionValue :type Boolean) (ElapsedSeconds :type "Float (double-precision)") (TriggeredSeconds :type "Float (double-precision)") (InputAction :type "InputAction Object Reference" :default "/Game/Blueprint/Input/Actions/IA_Handbrake.IA_Handbrake"))
  ;[1 1 1] Input
  (:`Started`
    (`self.DriftStart`))
  (:`Completed`
    (`self.DriftEnd`)))

(event `EnhancedInput|/Game/Blueprint/Input/Actions/IA_Boost`
  (params (ActionValue :type Boolean) (ElapsedSeconds :type "Float (double-precision)") (TriggeredSeconds :type "Float (double-precision)") (InputAction :type "InputAction Object Reference" :default "/Game/Blueprint/Input/Actions/IA_Boost.IA_Boost"))
  ;[1 1 1] Input
  (:`Triggered`
    (`self.SR_activateBoost`)))

(event `EnhancedInput|/Game/Blueprint/Input/Actions/IA_Throttle`
  (params (ActionValue :type Boolean) (ElapsedSeconds :type "Float (double-precision)") (TriggeredSeconds :type "Float (double-precision)") (InputAction :type "InputAction Object Reference" :default "/Game/Blueprint/Input/Actions/IA_Throttle.IA_Throttle"))
  (:`Triggered`
    (`self.AddMovementInput` (`self.GetActorForwardVector`))
    (`self.throttle` 1.0)))

(event `SR_activateBoost`
  ;[1 1 1] Input
  (`self.LocalActivateBoost`))

(event `LocalSteering`
  (params (axis :type "Float (double-precision)"))
  ;[1 1 1] Input
  (`self.SideAxis` axis))

(event `steering`
  (params (axisValue :type "Float (double-precision)"))
  ;[1 1 1] Input
  (`self.LocalSteering` axisValue))

(event `EnhancedInput|/Game/Blueprint/Input/Actions/IA_Steering`
  (params (ActionValue :type "Float (double-precision)") (ElapsedSeconds :type "Float (double-precision)") (TriggeredSeconds :type "Float (double-precision)") (InputAction :type "InputAction Object Reference" :default "/Game/Blueprint/Input/Actions/IA_Steering.IA_Steering"))
  ;[1 1 1] Input
  (:`Triggered`
    (`self.steering` ActionValue))
  (:`Completed`
    (`self.steering` 0.0)))

(event `EnhancedInput|/Game/Blueprint/Input/Actions/IA_Pause`
  (params (ActionValue :type Boolean) (ElapsedSeconds :type "Float (double-precision)") (TriggeredSeconds :type "Float (double-precision)") (InputAction :type "InputAction Object Reference" :default "/Game/Blueprint/Input/Actions/IA_Pause.IA_Pause"))
  (bind _returnvalue (`GameplayStatics.GetPlayerController` 0))
  (bind _returnvalue_2 (`GameplayStatics.GetPlayerController` 0))
  ;[1 1 1] Input
  (:`Triggered`
    (bind _asbp_lobby_player_controller (cast `/Game/Blueprint/PlayerController/BP_LobbyPlayerController` (`GameplayStatics.GetPlayerController` 0))
      (:`then`
        (bind _pausemenu (`/Game/Blueprint/PlayerController/BP_LobbyPlayerController.PauseMenu` _asbp_lobby_player_controller))
        (if (== (`Widget.GetVisibility` _pausemenu) 0)
          (set `Widget.Visibility` "Hidden" _pausemenu)
          (set `PlayerController.bShowMouseCursor` false _returnvalue)
          (else
            (set `Widget.Visibility` "Visible" _pausemenu)
            (set `PlayerController.bShowMouseCursor` true _returnvalue))))
      (:`CastFailed`
        (bind _asbp_track_player_controller (cast `/Game/Blueprint/PlayerController/BP_TrackPlayerController` (`GameplayStatics.GetPlayerController` 0)))
        (bind _pausemenu_2 (`/Game/Blueprint/PlayerController/BP_TrackPlayerController.PauseMenu` _asbp_track_player_controller))
        (if (== (`Widget.GetVisibility` _pausemenu_2) 0)
          (set `Widget.Visibility` "Hidden" _pausemenu_2)
          (set `PlayerController.bShowMouseCursor` false _returnvalue_2)
          (else
            (set `Widget.Visibility` "Visible" _pausemenu_2)
            (set `PlayerController.bShowMouseCursor` true _returnvalue_2)))))))

(event `self.ReceiveBeginPlay`
  (`parent.ReceiveBeginPlay`)
  (bind _outactors (`GameplayStatics.GetAllActorsOfClass` "/Game/EtienneTest/Maps/Blueprints/BP_SplineMeshTool.BP_SplineMeshTool_C"))
  (for _array_element _outactors
    (set `self.Track` (`self.GetComponentByClass` _array_element "/Script/Engine.SplineComponent")))
  (bind _outactors_2 (`GameplayStatics.GetAllActorsOfClass` "/Script/VroomVroomProject.CheckPoint"))
  (bind _output_get (set `self.checkpoint` _outactors_2))
  (`car.sort` _output_get))

(event `Freeze`
  ;[1 1 1] Input
  (`self.DisableInput` (`GameplayStatics.GetPlayerController` 0)))

(event `self.ReceiveTick`
  (params (DeltaSeconds :type "Float (single-precision)"))
  (`parent.ReceiveTick` DeltaSeconds)
  (`self.MesureLength`)
  (bind _asbp_track_game_mode (cast `/Game/Blueprint/GameMode/BP_TrackGameMode` (`GameplayStatics.GetGameMode`)))
  (`/Game/Blueprint/GameMode/BP_TrackGameMode.UpdateConstrollerPos` _asbp_track_game_mode self (`self.Dist`)))

(event `LocalActiveInvincible`
  (params (duration :type "Float (double-precision)"))
  (`PrimitiveComponent.SetMaterial` (`self.shipMesh_`) 0 "/Game/VGT/Demo/Materials/M_OrangeMaterial.M_OrangeMaterial")
  (`AbilityPawn.SetInvincible` duration))

(event `updateEnergy`
  (bind _returnvalue (`self.canBoost`))
  (bind _returnvalue_2 (`self.getEnergyRemaining`))
  (bind _asbp_track_player_controller (cast `/Game/Blueprint/PlayerController/BP_TrackPlayerController` (`GameplayStatics.GetPlayerController` 0)))
  (`/Game/Blueprint/PlayerController/BP_TrackPlayerController.updateEnergy` _asbp_track_player_controller _returnvalue (`KismetMathLibrary.FTrunc` _returnvalue_2)))

(event `ReceivePosition`
  (params (position :type Integer))
  (bind _asbp_track_player_controller (cast `/Game/Blueprint/PlayerController/BP_TrackPlayerController` (`GameplayStatics.GetPlayerController` 0)))
  (`/Game/Blueprint/PlayerController/BP_TrackPlayerController.updatePosition` _asbp_track_player_controller position))

(event `self.Miniaturize`
  (params (duration :type "Float (single-precision)"))
  (`parent.Miniaturize` duration)
  (set `self.desiredHeight_` 10.0)
  (set `FloatingPawnMovement.MaxSpeed` 2500.0 (`self.floatingPawnMovement_`)))

(event `LocalName`
  (params (name :type Integer))
  (bind _asplayer_name (cast `/Game/Blueprint/UI/PlayerName` (`WidgetComponent.GetUserWidgetObject` (`self.Widget`))))
  (`/Game/Blueprint/UI/PlayerName.SetName` _asplayer_name name)
  (bind _asplayer_name_2 (cast `/Game/Blueprint/UI/PlayerName` (`WidgetComponent.GetUserWidgetObject` (`self.Widget1`))))
  (`/Game/Blueprint/UI/PlayerName.SetName` _asplayer_name_2 name))

(event `self.SetVelocity`
  (params (value :type "Vector Structure"))
  (`PrimitiveComponent.SetPhysicsLinearVelocity` (`self.shipMesh_`) value false "None"))

(event `self.AddImpule`
  (params (value :type "Vector Structure"))
  (`PrimitiveComponent.AddImpulse` (`self.shipMesh_`) value "None" false))

(event `ActiveInvincible`
  (params (duration :type "Float (double-precision)"))
  (`self.LocalActiveInvincible` duration))

(event `incomingItem`
  (params (item :type "Item Class Reference"))
  (`AbilityPawn.PickItem` item))

(event `self.ResetMiniaturize`
  (`parent.ResetMiniaturize`)
  (set `self.desiredHeight_` 200.0)
  (set `FloatingPawnMovement.MaxSpeed` 5000.0 (`self.floatingPawnMovement_`)))

(event `ServerName`
  (params (name :type Integer))
  (`self.LocalName` name)
  (`self.Local`))

(event `Local`
  (`SceneComponent.SetHiddenInGame` (`self.Widget`) true false)
  (`SceneComponent.SetHiddenInGame` (`self.Widget1`) true false))

(event `self.DisableInvincible`
  (`parent.DisableInvincible`)
  (`PrimitiveComponent.SetMaterial` (`self.shipMesh_`) 0 "/Game/MarcTest/16833_go_kartMat.16833_go_kartMat"))

(event `setEnergyRecharge`
  (params (rate :type "Float (double-precision)"))
  (`self.SetEnergyChargeRate` rate))

(event `MultMiniaturize`
  (params (duration :type "Float (double-precision)"))
  (bind _returnvalue (`self.IsInvincible`))
  (if (not _returnvalue)
    (`AbilityPawn.Miniaturize` duration)))

(event `self.shipMesh_.OnComponentBeginOverlap`
  (params (OverlappedComponent :type "PrimitiveComponent Object Reference") (OtherActor :type "Actor Object Reference") (OtherComp :type "PrimitiveComponent Object Reference") (OtherBodyIndex :type Integer) (bFromSweep :type Boolean) (SweepResult :type "HitResult Structure (by ref)"))
  (bind _asbp_check_point (cast `/Game/Blueprint/Actor/BP_CheckPoint` OtherActor))
  (`|ExecutionSequence`
    (:`then_0`
      (if (== (+ (`self.SplineKey`) 1) (`KismetArrayLibrary.Array_Find` (`self.checkPoint`) _asbp_check_point))
        (bind _result (`/Engine/EditorBlueprintResources/StandardMacros.IncrementInt` (`self.SplineKey`))
          (:`  `
            (set `self.SplineKey` _result)
            (if (== _result (- (`KismetArrayLibrary.Array_Length` (`self.checkPoint`)) 1))
              (set `self.SplineKey` -1)
              (bind _result_2 (`/Engine/EditorBlueprintResources/StandardMacros.IncrementInt` (`self.Laps`))
                (:`  `
                  (set `self.Laps` _result_2)
                  (bind _asbp_track_player_controller (cast `/Game/Blueprint/PlayerController/BP_TrackPlayerController` (`GameplayStatics.GetPlayerController` 0)))
                  (`/Game/Blueprint/PlayerController/BP_TrackPlayerController.updateLaps` _asbp_track_player_controller _result_2)
                  (bind _asbp_track_game_mode (cast `/Game/Blueprint/GameMode/BP_TrackGameMode` (`GameplayStatics.GetGameMode`)))
                  (bind _output_get (set `self.isFinish` (== (`/Game/Blueprint/GameMode/BP_TrackGameMode.totalLaps` _asbp_track_game_mode) (`self.Laps`))))
                  (if _output_get
                    (`self.ChangeCamera` self)
                    (`self.SetActorHiddenInGame` true)))))))))
    (:`then_1`
      (bind _asbp_track_game_mode_2 (cast `/Game/Blueprint/GameMode/BP_TrackGameMode` (`GameplayStatics.GetGameMode`)))
      (`/Game/Blueprint/GameMode/BP_TrackGameMode.updateControllerLaps` _asbp_track_game_mode_2 self (`self.Laps`) (`self.SplineKey`)))))

(fn `MesureLength`
  (bind _checkpoint (`self.checkPoint`))
  (set `self.Dist` (`KismetMathLibrary.Vector_Distance2D` (`self.K2_GetActorLocation` (`|GetArrayItem` _checkpoint (mod (+ (`self.SplineKey`) 1) (`KismetArrayLibrary.Array_Length` _checkpoint)))) (`self.K2_GetActorLocation`))))

(fn `UserConstructionScript`)