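; Lobby game mode that spawns players' selected pawns and moves the session to a chosen map.
; BeginPlay shows a launch-game widget for the first player controller.
; CountDown displays a timer on every lobby controller, waits the GameInstance delay, triggers transitions, stores the player count and runs servertravel.
; Spawn functions replace and possess pawns, either at a given transform or at a PlayerStart indexed by player count, which the controller saves.
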(event `CountDown`
  (params (map :type String))
  (for _array_element (`GameStateBase.PlayerArray` (`GameplayStatics.GetGameState`))
    (bind _asbp_lobby_player_controller (cast `/Game/Blueprint/PlayerController/BP_LobbyPlayerController` (`PlayerState.GetPlayerController` _array_element)))
    (`/Game/Blueprint/PlayerController/BP_LobbyPlayerController.ShowCountDownLobby` _asbp_lobby_player_controller))
  (bind _asbp_game_instance (cast `/Game/Blueprint/GameInstance/BP_GameInstance` (`GameplayStatics.GetGameInstance`)))
  (`KismetSystemLibrary.Delay` (`KismetMathLibrary.Conv_IntToDouble` (`/Game/Blueprint/GameInstance/BP_GameInstance.GameStartCountDown` _asbp_game_instance)))
  (`self.FadeOut`)
  (`self.TravelTo` map))

(event `TravelTo`
  (params (Map :type String))
  (`self.SetPlayerCount`)
  (`KismetSystemLibrary.ExecuteConsoleCommand` (`KismetStringLibrary.Concat_StrStr` "servertravel " Map) null))

(event `FadeOut`
  (for _array_element (`GameStateBase.PlayerArray` (`GameplayStatics.GetGameState`))
    (bind _asbp_lobby_player_controller (cast `/Game/Blueprint/PlayerController/BP_LobbyPlayerController` (`PlayerState.GetPlayerController` _array_element)))
    (`/Game/Blueprint/PlayerController/BP_LobbyPlayerController.TransitionMap` _asbp_lobby_player_controller)))

(event `self.ReceiveBeginPlay`
  (bind _returnvalue (`|CreateWidget` "/Game/Blueprint/UI/BP_LaunchGame.BP_LaunchGame_C" (`GameplayStatics.GetPlayerController` 0)))
  (`UserWidget.AddToViewport` _returnvalue 1))

(fn `FindPlayerSpwawn`
  (returns (Location :type "Transform Structure"))
  (bind _returnvalue (`self.GetNumPlayers` (`GameStateBase.AuthorityGameMode` (`GameplayStatics.GetGameState`))))
  (bind _outactors (`GameplayStatics.GetAllActorsOfClass` "/Script/Engine.PlayerStart"))
  (return (`self.GetTransform` (`|GetArrayItem` _outactors (- _returnvalue 1)))))

(fn `SetPlayerCount`
  (bind _asbp_game_instance (cast `/Game/Blueprint/GameInstance/BP_GameInstance` (`GameplayStatics.GetGameInstance`)))
  (set `/Game/Blueprint/GameInstance/BP_GameInstance.NumberOfPlayer` (`KismetArrayLibrary.Array_Length` (`GameStateBase.PlayerArray` (`GameplayStatics.GetGameState`))) _asbp_game_instance))

(fn `SpawnPlayer`
  (params (PlayerController :type "PlayerController Object Reference") (SelectedPawn :type "Pawn Class Reference"))
  (returns (NewParam :type "Pawn Object Reference"))
  (bind _returnvalue (`Controller.K2_GetPawn` PlayerController))
  (`/Engine/EditorBlueprintResources/StandardMacros.IsValid` _returnvalue
    (:`Is Valid`
      (`self.K2_DestroyActor` _returnvalue))
    (:`Is Not Valid`
      _))
  (bind _location (`self.FindPlayerSpwawn`))
  (bind _asbp_lobby_player_controller (cast `/Game/Blueprint/PlayerController/BP_LobbyPlayerController` PlayerController))
  (`/Game/Blueprint/PlayerController/BP_LobbyPlayerController.SaveSapwnPoint` _asbp_lobby_player_controller _location)
  (bind _returnvalue_2 (`|SpawnActorFromClass` SelectedPawn _location "Undefined" "OverrideRootScale" null null))
  (`Controller.Possess` PlayerController _returnvalue_2)
  (return _returnvalue_2))

(fn `SpawnPlayerAtLocation`
  (params (PlayerController :type "PlayerController Object Reference") (SelectedPawn :type "Pawn Class Reference") (Location :type "Transform Structure"))
  (returns (NewParam :type "Pawn Object Reference"))
  (`self.K2_DestroyActor` (`Controller.K2_GetPawn` PlayerController))
  (bind _returnvalue (`|SpawnActorFromClass` SelectedPawn Location "Undefined" "OverrideRootScale" null null))
  (`Controller.Possess` PlayerController _returnvalue)
  (return _returnvalue))

(fn `UserConstructionScript`)