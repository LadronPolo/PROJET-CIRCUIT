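; Multiplayer kart race game mode that runs a race from countdown to final scoreboard.
; Once the expected player count joins, it starts the countdown, builds a ranking array of kart pawns, then unfreezes players.
; Karts' lap, checkpoint and distance updates feed that array, which Tick sorts to send positions back.
; It also spawns pawns at PlayerStarts, switches cameras to unfinished racers, relays sounds and shows scores when everyone finishes.
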(event `self.K2_PostLogin`
  (params (NewPlayer :type "PlayerController Object Reference"))
  (bind _asbp_game_instance (cast `/Game/Blueprint/GameInstance/BP_GameInstance` (`GameplayStatics.GetGameInstance`) :!label _label))
  (if (== (`/Game/Blueprint/GameInstance/BP_GameInstance.NumberOfPlayer` _asbp_game_instance) (`KismetArrayLibrary.Array_Length` (`GameStateBase.PlayerArray` (`GameplayStatics.GetGameState`))))
    (`KismetSystemLibrary.Delay` 2.0)
    (`self.CountDown`)
    (`self.Play2DSound` "/Game/Sounds/RaceStart.RaceStart")
    (`self.AddPlayers`)))

(event `self.K2_OnSwapPlayerControllers`
  (params (OldPC :type "PlayerController Object Reference") (NewPC :type "PlayerController Object Reference"))
  (goto _label))

(event `CountDown`
  (bind _playerarray (`GameStateBase.PlayerArray` (`GameplayStatics.GetGameState`)))
  (for _array_element _playerarray
    (bind _asbp_track_player_controller (cast `/Game/Blueprint/PlayerController/BP_TrackPlayerController` (`PlayerState.GetPlayerController` _array_element)))
    (`/Game/Blueprint/PlayerController/BP_TrackPlayerController.ShowCountDowninGame` _asbp_track_player_controller)
    (`/Game/Blueprint/PlayerController/BP_TrackPlayerController.getTotalPlayer` _asbp_track_player_controller (`KismetArrayLibrary.Array_Length` _playerarray))
    (`/Game/Blueprint/PlayerController/BP_TrackPlayerController.getTotalLaps` _asbp_track_player_controller (`self.totalLaps`)))
  (bind _asbp_game_instance (cast `/Game/Blueprint/GameInstance/BP_GameInstance` (`GameplayStatics.GetGameInstance`)))
  (`KismetSystemLibrary.Delay` (`KismetMathLibrary.Conv_IntToDouble` (`/Game/Blueprint/GameInstance/BP_GameInstance.GameStartCountDown` _asbp_game_instance)))
  (`self.UnfreezePlayer`))

(event `UnfreezePlayer`
  (for _array_element (`GameStateBase.PlayerArray` (`GameplayStatics.GetGameState`))
    (bind _asbp_track_player_controller (cast `/Game/Blueprint/PlayerController/BP_TrackPlayerController` (`PlayerState.GetPlayerController` _array_element)))
    (`/Game/Blueprint/PlayerController/BP_TrackPlayerController.Unfreeze` _asbp_track_player_controller)))

(event `UpdateConstrollerPos`
  (params (pawn :type "Pawn Object Reference") (dist :type "Float (double-precision)"))
  (for (_array_element _array_index) (`self.PlayerRanking`)
    (if (== (`.playerController` (break `PlayerRanking` _array_element)) pawn)
      (`KismetArrayLibrary.Array_Set` (`self.PlayerRanking`) _array_index (make `PlayerRanking` (break `PlayerRanking` _array_element) (`.checkpoint` (break `PlayerRanking` _array_element)) dist (`.playerController` (break `PlayerRanking` _array_element)) (`.idx` (break `PlayerRanking` _array_element)))))))

(event `updateControllerLaps`
  (params (pawn :type "Pawn Object Reference") (laps :type "Integer (by ref)") (checkpoint :type "Integer (by ref)"))
  (for (_array_element _array_index) (`self.PlayerRanking`)
    (if (== (`.playerController` (break `PlayerRanking` _array_element)) pawn)
      (`KismetArrayLibrary.Array_Set` (`self.PlayerRanking`) _array_index (make `PlayerRanking` laps checkpoint (`.distance` (break `PlayerRanking` _array_element)) (`.playerController` (break `PlayerRanking` _array_element)) (`.idx` (break `PlayerRanking` _array_element)))))))

(event `self.ReceiveTick`
  (params (DeltaSeconds :type "Float (single-precision)"))
  (`self.GameFinish`)
  (`self.sort` (`self.PlayerRanking`) (`self.totalLaps`))
  (for (_array_element _array_index) (`self.PlayerRanking`)
    (bind _asbp_kart (cast `/Game/Blueprint/Actor/BP_Kart` (`.playerController` (break `PlayerRanking` _array_element))))
    (`/Game/Blueprint/Actor/BP_Kart.ReceivePosition` _asbp_kart (+ _array_index 1))))

(event `getTotalLaps`
  (params (laps :type Integer))
  (set `self.totalLaps` laps))

(event `FindCamera`
  (params (Player :type "Pawn Object Reference") (current :type "Pawn Object Reference (by ref)"))
  (for _array_element (`self.PlayerRanking`)
    (if (and (and (!= (break `PlayerRanking` _array_element) (`self.totalLaps`)) (!= (`.playerController` (break `PlayerRanking` _array_element)) Player)) (!= (`.playerController` (break `PlayerRanking` _array_element)) current))
      (bind _asbp_track_player_controller (cast `/Game/Blueprint/PlayerController/BP_TrackPlayerController` (`Pawn.GetController` Player)))
      (`/Game/Blueprint/PlayerController/BP_TrackPlayerController.ChangeCamera` _asbp_track_player_controller (`.playerController` (break `PlayerRanking` _array_element)))
      (break))))

(event `ShowScoreGame`
  (for _array_element (`GameStateBase.PlayerArray` (`GameplayStatics.GetGameState`))
    (bind _asbp_track_player_controller (cast `/Game/Blueprint/PlayerController/BP_TrackPlayerController` (`PlayerState.GetPlayerController` _array_element)))
    (`/Game/Blueprint/PlayerController/BP_TrackPlayerController.ShowScoreBoard` _asbp_track_player_controller (`self.PlayerRanking`))))

(event `PlayerFinish`
  (`/Engine/EditorBlueprintResources/StandardMacros.IncrementInt` (`self.PlayerFinished`)))

(event `Play2DSound`
  (params (Sound :type "SoundBase Object Reference"))
  (for _array_element (`GameStateBase.PlayerArray` (`GameplayStatics.GetGameState`))
    (bind _asbp_kart_pawn_base (cast `/Game/Blueprints/BP_KartPawnBase` (`Controller.K2_GetPawn` (`PlayerState.GetPlayerController` _array_element))))
    (`/Game/Blueprints/BP_KartPawnBase.PlayNew2DSound` _asbp_kart_pawn_base Sound)))

(event `Play3DSound`
  (params (Sound :type "SoundBase Object Reference") (location :type "Vector Structure"))
  (for _array_element (`GameStateBase.PlayerArray` (`GameplayStatics.GetGameState`))
    (bind _asbp_kart_pawn_base (cast `/Game/Blueprints/BP_KartPawnBase` (`Controller.K2_GetPawn` (`PlayerState.GetPlayerController` _array_element))))
    (`/Game/Blueprints/BP_KartPawnBase.PlayNew3DSound` _asbp_kart_pawn_base Sound location)))

(event `Play3DSoundOnActor`
  (params (Kart :type "/Game/Blueprint/Actor/BP_Kart Object Reference") (Sound :type "SoundBase Object Reference"))
  (`/Game/Blueprints/BP_KartPawnBase.PlayMultiCast3DSound` Kart Sound))

(fn `AddPlayers`
  (for _array_element (`GameStateBase.PlayerArray` (`GameplayStatics.GetGameState`))
    (bind _result (`/Engine/EditorBlueprintResources/StandardMacros.IncrementInt` (`self.playeridx2`))
      (:`  `
        (`KismetArrayLibrary.Array_Add` (`self.PlayerRanking`) (make `PlayerRanking` 0 -1 0.0 (`Controller.K2_GetPawn` (`PlayerState.GetPlayerController` _array_element)) _result))))))

(fn `FindPlayerController`
  (params (Pawn :type "Pawn Object Reference"))
  (returns (PlayerController :type "PlayerController Object Reference"))
  (for _array_element (`GameStateBase.PlayerArray` (`GameplayStatics.GetGameState`))
    (bind _returnvalue (`PlayerState.GetPlayerController` _array_element))
    (if (== (`Controller.K2_GetPawn` _returnvalue) Pawn)
      (return _returnvalue))))

(fn `FindPlayerSpwawn`
  (returns (Location :type "Transform Structure"))
  (bind _returnvalue (`self.GetNumPlayers` (`GameStateBase.AuthorityGameMode` (`GameplayStatics.GetGameState`))))
  (bind _outactors (`GameplayStatics.GetAllActorsOfClass` "/Script/Engine.PlayerStart"))
  (return (`self.GetTransform` (`|GetArrayItem` _outactors (- _returnvalue 1)))))

(fn `GameFinish`
  (if (`self.IsGameFinish`)
    _
    (elif (== (`self.PlayerFinished`) (`GameplayStatics.GetNumPlayerStates`))
      (set `self.IsGameFinish` true)
      (`self.ShowScoreGame`))))

(fn `SpawnPlayer`
  (params (PlayerController :type "PlayerController Object Reference") (SelectedPawn :type "Pawn Class Reference"))
  (returns (pawn :type "Pawn Object Reference") (idx :type Integer))
  (bind _returnvalue (`Controller.K2_GetPawn` PlayerController))
  (`/Engine/EditorBlueprintResources/StandardMacros.IsValid` _returnvalue
    (:`Is Valid`
      (`self.K2_DestroyActor` _returnvalue))
    (:`Is Not Valid`
      _))
  (bind _location (`self.FindPlayerSpwawn`))
  (bind _returnvalue_2 (`|SpawnActorFromClass` SelectedPawn _location "Undefined" "OverrideRootScale" null null))
  (`Controller.Possess` PlayerController _returnvalue_2)
  (bind _result (`/Engine/EditorBlueprintResources/StandardMacros.IncrementInt` (`self.PlayerIdx`))
    (:`  `
      (return _returnvalue_2 _result))))

(fn `UserConstructionScript`)