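; Player controller for kart races that spawns the player's selected car and owns the race UI.
; On local BeginPlay it requests a frozen kart from the track game mode, creates the HUD and hidden pause menu, and adds input mapping.
; Local Tick updates speed, laps and kart energy.
; Events and functions relay race stats, items and timed oil overlay to the HUD, and handle countdown, input unfreeze and fade-out.
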(event `self.ReceiveBeginPlay`
  (if (`self.IsLocalPlayerController`)
    (bind _asbp_game_instance (cast `/Game/Blueprint/GameInstance/BP_GameInstance` (`GameplayStatics.GetGameInstance`)))
    (`self.SR_SpawnPlayer` (`/Game/Blueprint/GameInstance/BP_GameInstance.CarSelected` _asbp_game_instance))
    (`self.setupHUD`)
    (`self.setupInput`)))

(event `SR_SpawnPlayer`
  (params (SelectedPawn :type "Pawn Class Reference"))
  (bind _asbp_track_game_mode (cast `/Game/Blueprint/GameMode/BP_TrackGameMode` (`GameplayStatics.GetGameMode`)))
  (bind _pawn (`/Game/Blueprint/GameMode/BP_TrackGameMode.SpawnPlayer` _asbp_track_game_mode self SelectedPawn))
  (bind _asbp_kart (cast `/Game/Blueprint/Actor/BP_Kart` _pawn))
  (`/Game/Blueprint/Actor/BP_Kart.Freeze` _asbp_kart))

(event `self.ReceiveTick`
  (params (DeltaSeconds :type "Float (single-precision)"))
  (if (`self.IsLocalPlayerController`)
    (`self.updateHUD`)
    (bind _asbp_kart (cast `/Game/Blueprint/Actor/BP_Kart` (`self.K2_GetPawn`)))
    (`/Game/Blueprint/Actor/BP_Kart.updateEnergy` _asbp_kart)))

(event `TransitionMap`
  (bind _outactor (`LevelSequencePlayer.CreateLevelSequencePlayer` "/Game/LevelSequence/FadeOut.FadeOut"))
  (`MovieSceneSequencePlayer.Play` (`LevelSequenceActor.SequencePlayer` _outactor))
  (`/Game/Blueprint/UI/VehicleUI.StartFade` (`self.VehicleHud`)))

(event `ShowCountDowninGame`
  (bind _returnvalue (`|CreateWidget` "/Game/Blueprint/UI/BP_CountDown.BP_CountDown_C"))
  (`UserWidget.AddToViewport` _returnvalue 0))

(event `Unfreeze`
  (`self.EnableInput` (`self.K2_GetPawn`) self))

(event `getTotalPlayer`
  (params (totalPlayer :type Integer))
  (`self.UpdateTotalPlayer` totalPlayer))

(event `getTotalLaps`
  (params (totalLaps :type Integer))
  (`self.updateTotalLaps` totalLaps))

(event `updateItem`
  (params (image :type "Texture2D Object Reference"))
  (bind _vehiclehud (`self.VehicleHud`))
  (`/Engine/EditorBlueprintResources/StandardMacros.IsValid` _vehiclehud
    (:`Is Valid`
      (`/Game/Blueprint/UI/VehicleUI.updateItem` _vehiclehud image))))

(event `updateViewHuile`
  (params (duration :type "Float (double-precision)"))
  (bind _vehiclehud (`self.VehicleHud`))
  (`/Game/Blueprint/UI/VehicleUI.UpdateHuileView` _vehiclehud true)
  (`KismetSystemLibrary.Delay` duration)
  (`/Game/Blueprint/UI/VehicleUI.UpdateHuileView` _vehiclehud false))

(fn `setupHUD`
  (bind _returnvalue (`|CreateWidget` "/Game/Blueprint/UI/VehicleUI.VehicleUI_C" self))
  (bind _output_get (set `self.VehicleHud` _returnvalue))
  (`UserWidget.AddToViewport` _output_get 0)
  (bind _returnvalue_2 (`|CreateWidget` "/Game/Blueprint/UI/BP_PauseMenu.BP_PauseMenu_C"))
  (bind _output_get_2 (set `self.PauseMenu` _returnvalue_2))
  (`UserWidget.AddToViewport` _output_get_2 0)
  (`Widget.SetVisibility` (`self.PauseMenu`) "Hidden"))

(fn `setupInput`
  (`EnhancedInputSubsystemInterface.AddMappingContext` (subsystem `EnhancedInputLocalPlayerSubsystem`) "/Game/Blueprint/Input/IMC_Default.IMC_Default" 0 (struct)) ; Adding the Input Mapping Context needed to trigger the proper Input Actions.
)

(fn `setupMovementComponent`
  (bind _returnvalue (`self.K2_GetPawn`))
  (`/Engine/EditorBlueprintResources/StandardMacros.IsValid` _returnvalue
    (:`Is Valid`
      (set `self.body` _returnvalue))))

(fn `updateEnergy`
  (params (canBoost :type Boolean) (energy :type Integer))
  (bind _vehiclehud (`self.VehicleHud`))
  (`/Engine/EditorBlueprintResources/StandardMacros.IsValid` _vehiclehud
    (:`Is Valid`
      (`/Game/Blueprint/UI/VehicleUI.updateEnergy` _vehiclehud canBoost energy))))

(fn `updateHUD`
  (bind _vehiclehud (`self.VehicleHud`))
  (bind _body (`self.body`))
  (`/Engine/EditorBlueprintResources/StandardMacros.IsValid` (`self.body`)
    (:`Is Valid`
      (`/Engine/EditorBlueprintResources/StandardMacros.IsValid` _vehiclehud
        (:`Is Valid`
          (`/Game/Blueprint/UI/VehicleUI.UpdateSpeed` _vehiclehud (`KismetMathLibrary.Dot_VectorVector` (`self.GetVelocity` _body) (`self.GetActorForwardVector` _body)))
          (bind _asbp_kart (cast `/Game/Blueprint/Actor/BP_Kart` (`self.body`)))
          (`/Game/Blueprint/UI/VehicleUI.updateLaps` (`self.VehicleHud`) (`/Game/Blueprint/Actor/BP_Kart.Laps` _asbp_kart)))))
    (:`Is Not Valid`
      (`self.setupMovementComponent`))))

(fn `updateLaps`
  (params (Laps :type Integer))
  (bind _vehiclehud (`self.VehicleHud`))
  (`/Engine/EditorBlueprintResources/StandardMacros.IsValid` _vehiclehud
    (:`Is Valid`
      (`/Game/Blueprint/UI/VehicleUI.updateLaps` _vehiclehud Laps))))

(fn `updatePosition`
  (params (position :type Integer))
  (bind _vehiclehud (`self.VehicleHud`))
  (`/Engine/EditorBlueprintResources/StandardMacros.IsValid` _vehiclehud
    (:`Is Valid`
      (`/Game/Blueprint/UI/VehicleUI.updatePosition` _vehiclehud position))))

(fn `updateTotalLaps`
  (params (total :type Integer))
  (bind _vehiclehud (`self.VehicleHud`))
  (`/Engine/EditorBlueprintResources/StandardMacros.IsValid` _vehiclehud
    (:`Is Valid`
      (`/Game/Blueprint/UI/VehicleUI.updateTotalLaps` _vehiclehud total))))

(fn `UpdateTotalPlayer`
  (params (total :type Integer))
  (bind _vehiclehud (`self.VehicleHud`))
  (`/Engine/EditorBlueprintResources/StandardMacros.IsValid` _vehiclehud
    (:`Is Valid`
      (`/Game/Blueprint/UI/VehicleUI.updateTotalPlayer` _vehiclehud total))))

(fn `UserConstructionScript`)