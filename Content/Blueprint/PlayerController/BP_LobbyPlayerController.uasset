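; Player controller for the lobby that spawns the player's chosen car and manages the vehicle HUD.
; On local BeginPlay it passes the GameInstance's selected car to the lobby GameMode for spawning, creates the HUD and hidden pause menu, and adds the input mapping context.
; Tick caches the controlled pawn and feeds its forward speed to the HUD.
; Events show a countdown widget and play a fade-out sequence for map transitions.
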(event `self.ReceiveBeginPlay`
  (if (`self.IsLocalPlayerController`)
    (bind _asbp_game_instance (cast `/Game/Blueprint/GameInstance/BP_GameInstance` (`GameplayStatics.GetGameInstance`)))
    (`self.SR_SpawnPlayer` (`/Game/Blueprint/GameInstance/BP_GameInstance.CarSelected` _asbp_game_instance))
    (`self.setupHUD`)
    (`self.setupInput`)))

(event `SR_SpawnPlayer`
  (params (SelectedPawn :type "Pawn Class Reference"))
  (bind _asbp_lobby_game_mode (cast `/Game/Blueprint/GameMode/BP_LobbyGameMode` (`GameplayStatics.GetGameMode`)))
  (`/Game/Blueprint/GameMode/BP_LobbyGameMode.SpawnPlayer` _asbp_lobby_game_mode self SelectedPawn))

(event `self.ReceiveTick`
  (params (DeltaSeconds :type "Float (single-precision)"))
  (if (`self.IsLocalPlayerController`)
    (`self.updateHUD`)))

(event `TransitionMap`
  (bind _outactor (`LevelSequencePlayer.CreateLevelSequencePlayer` "/Game/LevelSequence/FadeOut.FadeOut"))
  (`MovieSceneSequencePlayer.Play` (`LevelSequenceActor.SequencePlayer` _outactor))
  (`/Game/Blueprint/UI/VehicleUI.StartFade` (`self.VehicleHud`)))

(event `ShowCountDownLobby`
  (bind _returnvalue (`|CreateWidget` "/Game/Blueprint/UI/BP_CountDownLobby.BP_CountDownLobby_C"))
  (`UserWidget.AddToViewport` _returnvalue 0))

(fn `setupHUD`
  (bind _returnvalue (`|CreateWidget` "/Game/Blueprint/UI/VehicleUI.VehicleUI_C" self))
  (bind _output_get (set `self.VehicleHud` _returnvalue))
  (`UserWidget.AddToViewport` _output_get 0)
  (bind _returnvalue_2 (`|CreateWidget` "/Game/Blueprint/UI/BP_PauseMenu.BP_PauseMenu_C"))
  (bind _output_get_2 (set `self.PauseMenu` _returnvalue_2))
  (`UserWidget.AddToViewport` _output_get_2 0)
  (`Widget.SetVisibility` (`self.PauseMenu`) "Hidden"))

(fn `setupInput`
  (`EnhancedInputSubsystemInterface.AddMappingContext` (subsystem `EnhancedInputLocalPlayerSubsystem`) "/Game/Blueprint/Input/IMC_Default.IMC_Default" 0 (struct)) ; Adding the Input Mapping Context needed to trigger the proper Input Actions.
)

(fn `setupMovementComponent`
  (bind _returnvalue (`self.K2_GetPawn`))
  (`/Engine/EditorBlueprintResources/StandardMacros.IsValid` _returnvalue
    (:`Is Valid`
      (bind _output_get (set `self.body` _returnvalue)))))

(fn `updateHUD`
  (bind _vehiclehud (`self.VehicleHud`))
  (bind _body (`self.body`))
  (`/Engine/EditorBlueprintResources/StandardMacros.IsValid` (`self.body`)
    (:`Is Valid`
      (`/Engine/EditorBlueprintResources/StandardMacros.IsValid` _vehiclehud
        (:`Is Valid`
          (`/Game/Blueprint/UI/VehicleUI.UpdateSpeed` _vehiclehud (`KismetMathLibrary.Dot_VectorVector` (`self.GetVelocity` _body) (`self.GetActorForwardVector` _body))))))
    (:`Is Not Valid`
      (`self.setupMovementComponent`))))

(fn `UserConstructionScript`)