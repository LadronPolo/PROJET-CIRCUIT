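; LobbyKart is the kart Blueprint for the lobby, adding pause-menu input on top of its parent class.
; BeginPlay runs the parent logic, then calls RestoreInput.
; IA_Pause casts player controller 0 to BP_LobbyPlayerController and checks its PauseMenu visibility.
; As wired, an already Visible menu stays Visible with the cursor shown, while any other state sets it Hidden with the cursor off, so it does not toggle.
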(event `EnhancedInput|/Game/Blueprint/Input/Actions/IA_Pause`
  (params (ActionValue :type Boolean) (ElapsedSeconds :type "Float (double-precision)") (TriggeredSeconds :type "Float (double-precision)") (InputAction :type "InputAction Object Reference" :default "/Game/Blueprint/Input/Actions/IA_Pause.IA_Pause"))
  (bind _returnvalue (`GameplayStatics.GetPlayerController` 0))
  (:`Triggered`
    (bind _asbp_lobby_player_controller (cast `/Game/Blueprint/PlayerController/BP_LobbyPlayerController` (`GameplayStatics.GetPlayerController` 0)))
    (bind _pausemenu (`/Game/Blueprint/PlayerController/BP_LobbyPlayerController.PauseMenu` _asbp_lobby_player_controller))
    (if (== (`Widget.GetVisibility` _pausemenu) 0)
      (set `Widget.Visibility` "Visible" _pausemenu)
      (set `PlayerController.bShowMouseCursor` true _returnvalue)
      (else
        (set `Widget.Visibility` "Hidden" _pausemenu)
        (set `PlayerController.bShowMouseCursor` false _returnvalue)))))

(event `self.ReceiveBeginPlay`
  (`parent.ReceiveBeginPlay`)
  (`AbilityPawn.RestoreInput`))

(fn `UserConstructionScript`
  (`parent.UserConstructionScript`))