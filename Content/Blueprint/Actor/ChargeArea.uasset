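; ChargeArea is a trigger zone actor that recharges a kart's energy while its car is inside the box.
; Box begin and end overlaps filter for car actors and pass them to the SR begin and end recharge events.
; These events use BP_TrackGameMode to find the car's player controller, then set the energy recharge on its controlled BP_Kart to ChargeRate on entry and zero on exit.
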(event `self.Box.OnComponentBeginOverlap`
  (params (OverlappedComponent :type "PrimitiveComponent Object Reference") (OtherActor :type "Actor Object Reference") (OtherComp :type "PrimitiveComponent Object Reference") (OtherBodyIndex :type Integer) (bFromSweep :type Boolean) (SweepResult :type "HitResult Structure (by ref)"))
  (bind _ascar (cast `car` OtherActor))
  (`self.SR_BeginRecharge` _ascar))

(event `SR_BeginRecharge`
  (params (actor :type "car Object Reference"))
  (bind _asbp_track_game_mode (cast `/Game/Blueprint/GameMode/BP_TrackGameMode` (`GameplayStatics.GetGameMode`)))
  (bind _playercontroller (`/Game/Blueprint/GameMode/BP_TrackGameMode.FindPlayerController` _asbp_track_game_mode actor))
  (bind _asbp_kart (cast `/Game/Blueprint/Actor/BP_Kart` (`Controller.K2_GetPawn` _playercontroller)))
  (`/Game/Blueprint/Actor/BP_Kart.setEnergyRecharge` _asbp_kart (`self.ChargeRate`)))

(event `self.Box.OnComponentEndOverlap`
  (params (OverlappedComponent :type "PrimitiveComponent Object Reference") (OtherActor :type "Actor Object Reference") (OtherComp :type "PrimitiveComponent Object Reference") (OtherBodyIndex :type Integer))
  (bind _ascar (cast `car` OtherActor))
  (`self.SR_EndRecharge` _ascar))

(event `SR_EndRecharge`
  (params (actor :type "car Object Reference"))
  (bind _asbp_track_game_mode (cast `/Game/Blueprint/GameMode/BP_TrackGameMode` (`GameplayStatics.GetGameMode`)))
  (bind _playercontroller (`/Game/Blueprint/GameMode/BP_TrackGameMode.FindPlayerController` _asbp_track_game_mode actor))
  (bind _asbp_kart (cast `/Game/Blueprint/Actor/BP_Kart` (`Controller.K2_GetPawn` _playercontroller)))
  (`/Game/Blueprint/Actor/BP_Kart.setEnergyRecharge` _asbp_kart 0.0))

(fn `UserConstructionScript`)