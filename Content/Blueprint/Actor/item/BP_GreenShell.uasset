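; BP_GreenShell is the green shell kart item, a projectile that travels straight and bounces off surfaces.
; On spawn it finds its owning kart's player controller through the track game mode and updates that controller's item.
; Tick drives velocity along the mesh's forward vector until the first bounce, then aligns the mesh to the velocity.
; Bounces play a 3D sound, and overlapping a kart only plays a 2D hit sound on it.
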(event `self.ReceiveBeginPlay`
  (bind _asbp_kart (cast `/Game/Blueprint/Actor/BP_Kart` (`self.GetOwner`)))
  (bind _asbp_track_game_mode (cast `/Game/Blueprint/GameMode/BP_TrackGameMode` (`GameplayStatics.GetGameMode`)))
  (bind _playercontroller (`/Game/Blueprint/GameMode/BP_TrackGameMode.FindPlayerController` _asbp_track_game_mode _asbp_kart))
  (bind _asbp_track_player_controller (cast `/Game/Blueprint/PlayerController/BP_TrackPlayerController` _playercontroller))
  (`/Game/Blueprint/PlayerController/BP_TrackPlayerController.updateItem` _asbp_track_player_controller "/Game/Images/GreenShell.GreenShell"))

(event `self.ReceiveTick`
  (params (DeltaSeconds :type "Float (single-precision)"))
  (bind _projectilemovementcomponent (`self.ProjectileMovementComponent`))
  (bind _mesh (`self.Mesh`))
  (if (`self.bounce`)
    (`SceneComponent.K2_SetWorldRotation` _mesh (`KismetMathLibrary.MakeRotationFromAxes` (`MovementComponent.Velocity` _projectilemovementcomponent)) false false)
    (else
      (set `MovementComponent.Velocity` (* (`SceneComponent.GetForwardVector` _mesh) (`self.Speed`)) _projectilemovementcomponent))))

(event `self.ProjectileMovementComponent.OnProjectileBounce`
  (params (ImpactResult :type "HitResult Structure (by ref)") (ImpactVelocity :type "Vector Structure (by ref)"))
  (set `self.bounce` true)
  (bind _asbp_track_game_mode (cast `/Game/Blueprint/GameMode/BP_TrackGameMode` (`GameplayStatics.GetGameMode`)))
  (`/Game/Blueprint/GameMode/BP_TrackGameMode.Play3DSound` _asbp_track_game_mode (`self.BounceSound`) ImpactResult_Location))

(event `self.Mesh.OnComponentBeginOverlap`
  (params (OverlappedComponent :type "PrimitiveComponent Object Reference") (OtherActor :type "Actor Object Reference") (OtherComp :type "PrimitiveComponent Object Reference") (OtherBodyIndex :type Integer) (bFromSweep :type Boolean) (SweepResult :type "HitResult Structure (by ref)"))
  (bind _asbp_kart_pawn_base (cast `/Game/Blueprints/BP_KartPawnBase` OtherActor))
  (`/Game/Blueprints/BP_KartPawnBase.PlayNew2DSound` _asbp_kart_pawn_base (`self.HitSound`)))

(fn `UserConstructionScript`)