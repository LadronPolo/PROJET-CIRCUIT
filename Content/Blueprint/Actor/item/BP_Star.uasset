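; BP_Star is the Super Star item actor for the kart racer, granting invincibility to the kart that owns it.
; On BeginPlay it casts its owner to BP_Kart, has BP_TrackGameMode find that kart's player controller, and updates the controller's item to Super_Star.
; Its Execute event calls ActiveInvincible on the owning kart, leaving the invincibility behavior to the kart itself.
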(event `self.ReceiveBeginPlay`
  (bind _asbp_kart (cast `/Game/Blueprint/Actor/BP_Kart` (`self.GetOwner`)))
  (bind _asbp_track_game_mode (cast `/Game/Blueprint/GameMode/BP_TrackGameMode` (`GameplayStatics.GetGameMode`)))
  (bind _playercontroller (`/Game/Blueprint/GameMode/BP_TrackGameMode.FindPlayerController` _asbp_track_game_mode _asbp_kart))
  (bind _asbp_track_player_controller (cast `/Game/Blueprint/PlayerController/BP_TrackPlayerController` _playercontroller))
  (`/Game/Blueprint/PlayerController/BP_TrackPlayerController.updateItem` _asbp_track_player_controller "/Game/Images/Super_Star.Super_Star"))

(event `self.Execute`
  (bind _asbp_kart (cast `/Game/Blueprint/Actor/BP_Kart` (`self.GetOwner`)))
  (`/Game/Blueprint/Actor/BP_Kart.ActiveInvincible` _asbp_kart (`self.invincible`)))

(fn `UserConstructionScript`)