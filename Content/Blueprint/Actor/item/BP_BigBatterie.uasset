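; BP_BigBatterie is a kart item actor that grants its owning kart battery energy when used.
; On BeginPlay it updates the owner's player controller item display to BatteriePack, has the game mode change its mesh material, and snaps itself to the owner's "Fiole" skeletal socket.
; Execute adds energy over a duration, plays a sound, briefly flashes an activation overlay material on the kart body, then destroys the actor.
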(event `self.ReceiveBeginPlay`
  (bind _returnvalue (`self.GetOwner`))
  (`|ExecutionSequence`
    (:`then_0`
      (bind _asbp_kart (cast `/Game/Blueprint/Actor/BP_Kart` _returnvalue))
      (bind _asbp_track_game_mode (cast `/Game/Blueprint/GameMode/BP_TrackGameMode` (`GameplayStatics.GetGameMode`)))
      (bind _playercontroller (`/Game/Blueprint/GameMode/BP_TrackGameMode.FindPlayerController` _asbp_track_game_mode _asbp_kart))
      (bind _asbp_track_player_controller (cast `/Game/Blueprint/PlayerController/BP_TrackPlayerController` _playercontroller))
      (`/Game/Blueprint/PlayerController/BP_TrackPlayerController.updateItem` _asbp_track_player_controller "/Game/Images/BatteriePack.BatteriePack")
      (bind _asbp_track_game_mode_2 (cast `/Game/Blueprint/GameMode/BP_TrackGameMode` (`GameplayStatics.GetGameMode`)))
      (`/Game/Blueprint/GameMode/BP_TrackGameMode.ChangeMaterial` _asbp_track_game_mode_2 1.0 (`self.StaticMesh`)))
    (:`then_1`
      (for _array_element (`self.K2_GetComponentsByClass` _returnvalue "/Script/Engine.SkeletalMeshComponent")
        (`/Engine/EditorBlueprintResources/StandardMacros.IsValid` _array_element
          (:`Is Valid`
            (if (`SceneComponent.DoesSocketExist` _array_element "Fiole")
              (`self.K2_AttachToComponent` _array_element "Fiole" "SnapToTarget" "KeepWorld" "KeepWorld"))))))))

(event `self.Execute`
  (bind _asbp_kart (cast `/Game/Blueprint/Actor/BP_Kart` (`self.GetOwner`)))
  (`/Game/Blueprint/Actor/BP_Kart.addEnergyBattery` _asbp_kart (`self.energy`) (`self.duration`))
  (`GameplayStatics.PlaySound2D` (`self.Sound`) 1.0 1.0 0.0 null null)
  (bind _body (`/Game/Blueprints/BP_KartPawnBase.Body` _asbp_kart))
  (`MeshComponent.SetOverlayMaterial` _body "/Game/Artist_Folder/VFX_Tristan_New/Materials/MI_Item_StarActivation_Big.MI_Item_StarActivation_Big")
  (`KismetSystemLibrary.Delay` 1.5)
  (`MeshComponent.SetOverlayMaterial` _body null)
  (`self.K2_DestroyActor`))

(fn `UserConstructionScript`)