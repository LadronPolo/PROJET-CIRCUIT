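; BP_Banana is a droppable kart-race item that briefly freezes the input of cars that hit it.
; On spawn it reports itself to the owning kart's player controller and attaches to the owner's Shell socket.
; Execute detaches it and clears the owner a second later, ending the owner's immunity to it.
; Overlapping a car freezes that car and destroys the banana, while overlapping another item destroys both.
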(event `self.ReceiveBeginPlay`
  (bind _returnvalue (`self.GetOwner`))
  (`|ExecutionSequence`
    (:`then_0`
      (bind _asbp_kart (cast `/Game/Blueprint/Actor/BP_Kart` _returnvalue))
      (bind _asbp_track_game_mode (cast `/Game/Blueprint/GameMode/BP_TrackGameMode` (`GameplayStatics.GetGameMode`)))
      (bind _playercontroller (`/Game/Blueprint/GameMode/BP_TrackGameMode.FindPlayerController` _asbp_track_game_mode _asbp_kart))
      (bind _asbp_track_player_controller (cast `/Game/Blueprint/PlayerController/BP_TrackPlayerController` _playercontroller))
      (`/Game/Blueprint/PlayerController/BP_TrackPlayerController.updateItem` _asbp_track_player_controller "/Game/Images/Banana.Banana"))
    (:`then_1`
      (`self.K2_AttachToActor` _returnvalue "Shell" "SnapToTarget" "KeepWorld" "KeepWorld"))))

(event `self.Execute`
  (cast `/Game/Blueprint/Actor/BP_Kart` (`self.GetOwner`))
  (`self.K2_DetachFromActor` "KeepWorld" "KeepWorld" "KeepWorld")
  (`KismetSystemLibrary.Delay` 1.0)
  (`self.SetOwner` null))

(event `self.StaticMesh.OnComponentBeginOverlap`
  (params (OverlappedComponent :type "PrimitiveComponent Object Reference") (OtherActor :type "Actor Object Reference") (OtherComp :type "PrimitiveComponent Object Reference") (OtherBodyIndex :type Integer) (bFromSweep :type Boolean) (SweepResult :type "HitResult Structure (by ref)"))
  (if (!= OtherActor (`self.GetOwner`))
    (bind _ascar (cast `car` OtherActor)
      (:`then`
        (`AbilityPawn.FreezeInput` _ascar (`self.duration`))
        (`self.K2_DestroyActor`))
      (:`CastFailed`
        (bind _asitem (cast `Item` OtherActor))
        (`self.K2_DestroyActor`)
        (`self.K2_DestroyActor` _asitem)))))

(fn `UserConstructionScript`)