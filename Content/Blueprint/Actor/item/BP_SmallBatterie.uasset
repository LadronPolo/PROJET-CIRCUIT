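; Small battery item actor owned by a kart, which restores energy to that kart when executed.
; On BeginPlay it finds the owning kart's player controller through BP_TrackGameMode and updates its current item to Batterie.
; Execute adds the Energy amount to the owning kart and plays a 2D sound.
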(event `self.ReceiveBeginPlay`
  (bind _asbp_kart (cast `/Game/Blueprint/Actor/BP_Kart` (`self.GetOwner`)))
  (bind _asbp_track_game_mode (cast `/Game/Blueprint/GameMode/BP_TrackGameMode` (`GameplayStatics.GetGameMode`)))
  (bind _playercontroller (`/Game/Blueprint/GameMode/BP_TrackGameMode.FindPlayerController` _asbp_track_game_mode _asbp_kart))
  (bind _asbp_track_player_controller (cast `/Game/Blueprint/PlayerController/BP_TrackPlayerController` _playercontroller))
  (`/Game/Blueprint/PlayerController/BP_TrackPlayerController.updateItem` _asbp_track_player_controller "/Game/Images/Batterie.Batterie"))

(event `self.Execute`
  (bind _asbp_kart (cast `/Game/Blueprint/Actor/BP_Kart` (`self.GetOwner`)))
  (`AbilityPawn.AddEnergy` _asbp_kart (`self.energy`))
  (`GameplayStatics.PlaySound2D` (`self.Sound`) 1.0 1.0 0.0 null null))

(fn `UserConstructionScript`)