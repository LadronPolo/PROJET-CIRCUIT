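; Oil (Huile) kart item that obscures the view of every player except its user.
; On BeginPlay it reports itself to the owning kart's track controller and attaches to the "Fiole" socket on the owner's skeletal mesh.
; Execute loops the PlayerArray, triggering each opponent's timed oil view and 2D sound, and playing the item animation through the game mode.
; Tick destroys the actor once the animation's Trail notify state has been active.
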(event `self.ReceiveBeginPlay`
  (bind _returnvalue (`self.GetOwner`))
  (`|ExecutionSequence`
    (:`then_0`
      (bind _asbp_kart (cast `/Game/Blueprint/Actor/BP_Kart` _returnvalue))
      (bind _asbp_track_game_mode (cast `/Game/Blueprint/GameMode/BP_TrackGameMode` (`GameplayStatics.GetGameMode`)))
      (bind _playercontroller (`/Game/Blueprint/GameMode/BP_TrackGameMode.FindPlayerController` _asbp_track_game_mode _asbp_kart))
      (bind _asbp_track_player_controller (cast `/Game/Blueprint/PlayerController/BP_TrackPlayerController` _playercontroller))
      (`/Game/Blueprint/PlayerController/BP_TrackPlayerController.updateItem` _asbp_track_player_controller "/Game/Images/Huile.Huile"))
    (:`then_1`
      (for _array_element (`self.K2_GetComponentsByClass` _returnvalue "/Script/Engine.SkeletalMeshComponent")
        (`/Engine/EditorBlueprintResources/StandardMacros.IsValid` _array_element
          (:`Is Valid`
            (if (`SceneComponent.DoesSocketExist` _array_element "Fiole")
              (`self.K2_AttachToComponent` _array_element "Fiole" "SnapToTarget" "KeepWorld" "KeepWorld"))))))))

(event `self.Execute`
  (bind _asbp_kart (cast `/Game/Blueprint/Actor/BP_Kart` (`self.GetOwner`)))
  (`self.loopAllPlayer` (`self.duration`) _asbp_kart))

(event `loopAllPlayer`
  (params (Duration :type "Float (double-precision)") (car :type "car Object Reference"))
  (for _array_element (`GameStateBase.PlayerArray` (`GameplayStatics.GetGameState`))
    (bind _returnvalue (`PlayerState.GetPlayerController` _array_element))
    (`/Engine/EditorBlueprintResources/StandardMacros.IsValid` _returnvalue
      (:`Is Valid`
        (bind _asbp_track_player_controller (cast `/Game/Blueprint/PlayerController/BP_TrackPlayerController` _returnvalue))
        (bind _returnvalue_2 (`Controller.K2_GetPawn` _returnvalue))
        (if (!= _returnvalue_2 car)
          (`/Game/Blueprint/PlayerController/BP_TrackPlayerController.updateViewHuile` _asbp_track_player_controller Duration)
          (bind _asbp_kart_pawn_base (cast `/Game/Blueprints/BP_KartPawnBase` _returnvalue_2))
          (`/Game/Blueprints/BP_KartPawnBase.PlayNew2DSound` _asbp_kart_pawn_base (`self.Sound`))
          (bind _asbp_track_game_mode (cast `/Game/Blueprint/GameMode/BP_TrackGameMode` (`GameplayStatics.GetGameMode`)))
          (`/Game/Blueprint/GameMode/BP_TrackGameMode.PlayAnim` _asbp_track_game_mode (`self.SkeletalMesh`)))))))

(event `self.ReceiveTick`
  (params (DeltaSeconds :type "Float (single-precision)"))
  (if (`AnimInstance.WasAnimNotifyStateActiveInAnyState` (`SkeletalMeshComponent.GetAnimInstance` (`self.SkeletalMesh`)) "/Script/Engine.AnimNotifyState_Trail")
    (`self.K2_DestroyActor`)))

(fn `UserConstructionScript`)