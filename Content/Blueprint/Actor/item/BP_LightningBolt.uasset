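; Lightning bolt item for the kart game that shrinks every other player's kart for a set duration.
; On BeginPlay it finds the owning kart's player controller through the track game mode and updates that player's item to LightningBolt.
; Execute loops over the game state's PlayerArray and calls MultMiniaturize on each controlled kart pawn except the owner.
; Players without a valid player controller are skipped.
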(event `self.ReceiveBeginPlay`
  (bind _asbp_kart (cast `/Game/Blueprint/Actor/BP_Kart` (`self.GetOwner`)))
  (bind _asbp_track_game_mode (cast `/Game/Blueprint/GameMode/BP_TrackGameMode` (`GameplayStatics.GetGameMode`)))
  (bind _playercontroller (`/Game/Blueprint/GameMode/BP_TrackGameMode.FindPlayerController` _asbp_track_game_mode _asbp_kart))
  (bind _asbp_track_player_controller (cast `/Game/Blueprint/PlayerController/BP_TrackPlayerController` _playercontroller))
  (`/Game/Blueprint/PlayerController/BP_TrackPlayerController.updateItem` _asbp_track_player_controller "/Game/Images/LightningBolt.LightningBolt"))

(event `self.Execute`
  (bind _asbp_kart (cast `/Game/Blueprint/Actor/BP_Kart` (`self.GetOwner`)))
  (`self.loopAllPlayer` (`self.duration`) _asbp_kart))

(event `loopAllPlayer`
  (params (Duration :type "Float (double-precision)") (car :type "car Object Reference"))
  (for _array_element (`GameStateBase.PlayerArray` (`GameplayStatics.GetGameState`))
    (bind _returnvalue (`PlayerState.GetPlayerController` _array_element))
    (`/Engine/EditorBlueprintResources/StandardMacros.IsValid` _returnvalue
      (:`Is Valid`
        (bind _asbp_kart_pawn_base (cast `/Game/Blueprints/BP_KartPawnBase` (`Controller.K2_GetPawn` _returnvalue)))
        (if (!= _asbp_kart_pawn_base car)
          (`/Game/Blueprints/BP_KartPawnBase.MultMiniaturize` _asbp_kart_pawn_base Duration))))))

(fn `UserConstructionScript`)